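; BP_Camera is the tower defense camera actor, which its construction script pins at a fixed height above the world origin.
; Enhanced Input rotate actions yaw the whole actor, while zoom actions set a clamped target field of view offset from the current one.
; Tick eases the camera's field of view toward that target and switches itself off on arrival until the next zoom input re-enables it.
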(event `EnhancedInput|/Game/TowerDefense/Input/Actions/IA_RotateCamera`
  (params (ActionValue :type "Float (double-precision)") (ElapsedSeconds :type "Float (double-precision)") (TriggeredSeconds :type "Float (double-precision)") (InputAction :type "InputAction Object Reference" :default "/Game/TowerDefense/Input/Actions/IA_RotateCamera.IA_RotateCamera"))
  (bind (_returnvalue_roll _returnvalue_pitch _returnvalue_yaw) (`KismetMathLibrary.BreakRotator` (`self.K2_GetActorRotation`)))
  ;[0.05469 0 1] Camera Rotation
  (:`Triggered`
    (`self.K2_SetActorRotation` (`KismetMathLibrary.MakeRotator` _returnvalue_roll _returnvalue_pitch (+ _returnvalue_yaw (/ ActionValue 2.0))))))

(event `EnhancedInput|/Game/TowerDefense/Input/Actions/IA_ZoomCamera`
  (params (ActionValue :type "Float (double-precision)") (ElapsedSeconds :type "Float (double-precision)") (TriggeredSeconds :type "Float (double-precision)") (InputAction :type "InputAction Object Reference" :default "/Game/TowerDefense/Input/Actions/IA_ZoomCamera.IA_ZoomCamera"))
  ;[1 0.3281 0] Camera Zoom
  (:`Triggered`
    (set `self.Desired Zoom` (`KismetMathLibrary.FClamp` (+ (* ActionValue 20.0) (`CameraComponent.FieldOfView` (`self.Camera`))) 40.0 120.0))
    (`self.SetActorTickEnabled` true)))

(event `self.ReceiveTick`
  (params (DeltaSeconds :type "Float (single-precision)"))
  (bind _desired_zoom (`self.Desired Zoom`))
  (bind _fieldofview (`CameraComponent.FieldOfView` (`self.Camera`)))
  ;[1 0.3281 0] Camera Zoom
  (if (== _fieldofview _desired_zoom)
    (`self.SetActorTickEnabled` false)
    (else
      (`CameraComponent.SetFieldOfView` (`self.Camera`) (`KismetMathLibrary.FInterpTo` _fieldofview _desired_zoom DeltaSeconds 2.0)))))

(fn `UserConstructionScript`
  (`self.K2_SetActorLocation` (0.0 0.0 2500.0)))