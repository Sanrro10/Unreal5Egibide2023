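; Tower defense game mode that tracks the player's health and money and shows both on the game interface widget.
; BeginPlay creates the widget, adds it to the viewport and calls the damage and money functions with zero to initialise its text.
; ReceiveDamage and AddMoney update their values and push them to the widget.
; When health drops to zero or below, LooseGame pauses the game and prints "Defeat".
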(event `self.ReceiveBeginPlay`
  (bind _returnvalue (`|CreateWidget` "/Game/TowerDefense/Blueprints/Widgets/WBP_GameInterface.WBP_GameInterface_C"))
  (bind _output_get (set `self.WBP_GameInterface` _returnvalue))
  (`UserWidget.AddToViewport` _output_get 0)
  (`self.Receive Damage` 0)
  (`self.Add Money` 0))

(fn `Add Money`
  (params (Money :type Integer))
  (bind _output_get (set `self.Money` (+ (`self.Money`) Money)))
  (`/Game/TowerDefense/Blueprints/Widgets/WBP_GameInterface.Update Money Text` (`self.WBP_GameInterface`) _output_get))

(fn `Loose Game`
  (`GameplayStatics.SetGamePaused` true)
  (`KismetSystemLibrary.PrintString` "Defeat" true true (struct :`R` 1.0 :`A` 1.0) 999.0))

(fn `Receive Damage`
  (params (Damage :type Integer))
  (bind _output_get (set `self.Health Points` (- (`self.Health Points`) Damage)))
  (`/Game/TowerDefense/Blueprints/Widgets/WBP_GameInterface.Update Health Text` (`self.WBP_GameInterface`) _output_get)
  (if (<= _output_get 0)
    (`self.Loose Game`)))

(fn `UserConstructionScript`)