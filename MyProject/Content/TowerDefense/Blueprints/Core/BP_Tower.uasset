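; Tower defense turret that fires homing projectiles at enemies inside its Sphere range.
; Sphere overlaps add and remove BP_BaseEnemy actors in the Enemies array, and the first entry starts a looping timer at RateOfFire.
; Each shot spawns at the Sphere and homes on the capsule of the first enemy in the array.
; An empty array clears the timer but leaves Shooting set, so firing does not restart.
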(event `self.Sphere.OnComponentBeginOverlap`
  (params (OverlappedComponent :type "PrimitiveComponent Object Reference") (OtherActor :type "Actor Object Reference") (OtherComp :type "PrimitiveComponent Object Reference") (OtherBodyIndex :type Integer) (bFromSweep :type Boolean) (SweepResult :type "HitResult Structure (by ref)"))
  (bind _asbp_base_enemy (cast `/Game/TowerDefense/Enemies/BP_BaseEnemy` OtherActor))
  (`KismetArrayLibrary.Array_Add` (`self.Enemies`) _asbp_base_enemy)
  (if (not (`self.Shooting`))
    (set `self.Shooting` true)
    (bind _returnvalue (`KismetSystemLibrary.K2_SetTimerDelegate` (delegate `Shoot`) (`self.Rate of Fire`) true))
    (set `self.Shoot Timer Handle` _returnvalue)))

(event `Shoot`
  (bind _returnvalue (`|SpawnActorFromClass` (`self.Projectile`) (`SceneComponent.K2_GetComponentToWorld` (`self.Sphere`)) "Undefined" "MultiplyWithRoot" null null))
  (set `ProjectileMovementComponent.HomingTargetComponent` (`Character.CapsuleComponent` (`|GetArrayItem` (`self.Enemies`))) (`/Game/TowerDefense/Blueprints/Core/BP_Projectile.ProjectileMovement` _returnvalue)))

(event `self.Sphere.OnComponentEndOverlap`
  (params (OverlappedComponent :type "PrimitiveComponent Object Reference") (OtherActor :type "Actor Object Reference") (OtherComp :type "PrimitiveComponent Object Reference") (OtherBodyIndex :type Integer))
  (bind _enemies (`self.Enemies`))
  (bind _asbp_base_enemy (cast `/Game/TowerDefense/Enemies/BP_BaseEnemy` OtherActor))
  (`KismetArrayLibrary.Array_RemoveItem` _enemies _asbp_base_enemy)
  (if (`KismetArrayLibrary.Array_IsEmpty` _enemies)
    (`KismetSystemLibrary.K2_ClearAndInvalidateTimerHandle` (`self.Shoot Timer Handle`))))

(fn `UserConstructionScript`)