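; Tower defense wave spawner that emits enemies in configured groups and sends each toward a Destination actor's location.
; Each SpawnerData entry sets a group's enemy class, count and delay until the next group.
; A single looping timer spawns at the spawner's transform, pauses between groups, resumes for the next one and is cleared after the last.
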(event `self.ReceiveBeginPlay`
  (`self.InitializeGroup`))

(event `InitializeGroup`
  (if (< (`self.GroupID`) (`KismetArrayLibrary.Array_Length` (`self.SpawnerData`)))
    (set `self.CurrentSpawnerData` (`|GetArrayItem` (`self.SpawnerData`) (`self.GroupID`)))
    (if (!= (`self.GroupID`) 0)
      (`KismetSystemLibrary.K2_UnPauseTimerHandle` (`self.SpawnerTimer`))
      (else
        (bind _returnvalue (`KismetSystemLibrary.K2_SetTimerDelegate` (delegate `SpawnEnemy`) (`self.SpawnerGeneralDelay`) true))
        (set `self.SpawnerTimer` _returnvalue)))
    (else
      (`KismetSystemLibrary.K2_ClearAndInvalidateTimerHandle` (`self.SpawnerTimer`)))))

(event `SpawnEnemy`
  (if (>= (`self.EnemyCount`) (`self.GetCurrentEnemyNum`))
    (`KismetSystemLibrary.K2_PauseTimerHandle` (`self.SpawnerTimer`))
    (`KismetSystemLibrary.Delay` (`self.GetCurrentGroupDelay`))
    (set `self.EnemyCount` 0)
    (`/Engine/EditorBlueprintResources/StandardMacros.IncrementInt` (`self.GroupID`)
      (:`  `
        (`self.InitializeGroup`)))
    (else
      (bind _returnvalue (`|SpawnActorFromClass` (`self.GetCurrentEnemyClass`) (`self.GetTransform`) "AdjustIfPossibleButAlwaysSpawn" "MultiplyWithRoot" null null))
      (set `/Game/TowerDefense/Enemies/BP_BaseEnemy.Goal Location` (`self.K2_GetActorLocation` (`self.Destination`)) _returnvalue)
      (`/Engine/EditorBlueprintResources/StandardMacros.IncrementInt` (`self.EnemyCount`)))))

(fn `GetCurrentEnemyClass`
  (returns (`Enemy Type` :type "/Game/TowerDefense/Enemies/BP_BaseEnemy Class Reference"))
  (return (`.EnemyType_5_00B293304A325654C19BBCB501C4F90F` (break `/Game/TowerDefense/Structures_Enumerators/S_EnemySpawnerData` (`self.CurrentSpawnerData`)))))

(fn `GetCurrentEnemyNum`
  (returns (`Num Enemies` :type Integer))
  (return (`.NumEnemies_2_9B4BB01541D1A85D3EB519BCE15E0356` (break `/Game/TowerDefense/Structures_Enumerators/S_EnemySpawnerData` (`self.CurrentSpawnerData`)))))

(fn `GetCurrentGroupDelay`
  (returns (`Delay Unltil Next Wave` :type "Float (double-precision)"))
  (return (`.DelayUnltilNextGroup_9_6358FEE74DE7A811917B8DA44B6DA8A5` (break `/Game/TowerDefense/Structures_Enumerators/S_EnemySpawnerData` (`self.CurrentSpawnerData`)))))

(fn `UserConstructionScript`)