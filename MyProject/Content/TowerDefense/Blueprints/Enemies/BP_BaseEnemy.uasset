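; BP_BaseEnemy is the base tower defense enemy, which moves to a goal, can damage the player's side and pays money when killed.
; On possession it caches its AIC_Enemy controller and, a tick later, has it move to the goal location.
; It reports to GM_TowerDefense: DealDamage passes on its damage and destroys it, while ReceiveDamage lowers health and awards money before destroying it at zero.
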(event `self.ReceivePossessed`
  (params (NewController :type "Controller Object Reference"))
  (bind _asaic_enemy (cast `/Game/TowerDefense/Blueprints/Enemies/AIC_Enemy` NewController))
  (set `self.AIController` _asaic_enemy)
  (`KismetSystemLibrary.DelayUntilNextTick`)
  (`self.MoveToGoalLocation` (`self.Goal Location`)))

(event `self.ReceiveBeginPlay`
  (bind _asgm_tower_defense (cast `/Game/TowerDefense/Blueprints/Core/GM_TowerDefense` (`GameplayStatics.GetGameMode`)))
  (set `self.GM Tower Defense` _asgm_tower_defense))

(fn `Deal Damage`
  (`/Game/TowerDefense/Blueprints/Core/GM_TowerDefense.Receive Damage` (`self.GM Tower Defense`) (`self.Damage`))
  (`self.K2_DestroyActor`))

(fn `MoveToGoalLocation`
  (params (`Goal Location` :type "Vector Structure"))
  (`/Game/TowerDefense/Blueprints/Enemies/AIC_Enemy.MoveToGoalLocation` (`self.AIController`) `Goal Location`))

(fn `Receive Damage`
  (params (Damage :type Integer))
  (bind _output_get (set `self.Health Points` (- (`self.Health Points`) Damage)))
  (if (<= _output_get 0)
    (`/Game/TowerDefense/Blueprints/Core/GM_TowerDefense.Add Money` (`self.GM Tower Defense`) (`self.Money`))
    (`self.K2_DestroyActor`)))

(fn `UserConstructionScript`)